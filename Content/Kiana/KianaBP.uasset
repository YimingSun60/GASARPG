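; Kiana character Blueprint that turns left mouse input into Gameplay Ability System melee attacks.
; A tap activates KianaMelee3 and a short hold activates KianaMelee3Branch, both only while CanInput is true.
; The LongHoldDetection macro separates the two using a retriggerable delay and two gates, firing Held without waiting for release.
; Unconnected leftover nodes hold InputState tag switching and a tag-printing debug timer.
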(event Custom|GetTag
  (for _array_element (.gameplaytags (GameplayTags|GetOwnedGameplayTags (Variables|Default|GetAbilitySystemComponent) :!class /Script/GameplayTags.GameplayTagAssetInterface))
    (Development|PrintString (Utilities|String|ToString(Name) (GameplayTags|GetTagName _array_element))))
  (Development|PrintString "------------------------------------------------------"))

(event EventBeginPlay)

(event Collision|EventActorBeginOverlap
  (params (OtherActor :type Actor%20Object%20Reference)))

(event EventTick
  (params (DeltaSeconds :type Float%20%28single-precision%29)))

(event Input|MouseEvents|LeftMouseButton
  (params (Key :type Key%20Structure :default "None"))
  (bind _caninput (Variables|Default|GetCanInput))
  (:Pressed
    (Utilities|LongHoldDetection 0.2 :!label _label
      (:Held
        (if _caninput
          (Abilities|TryActivateAbilitybyClass (Variables|Default|GetAbilitySystemComponent) "/Game/Kiana/Abilities/KianaMelee3Branch.KianaMelee3Branch_C" true)))
      (:Tapped
        (if _caninput
          (Abilities|TryActivateAbilitybyClass (Variables|Default|GetAbilitySystemComponent) "/Game/Kiana/Abilities/KianaMelee3.KianaMelee3_C" true)))))
  (:Released
    (goto _label Released)))

(fn ConstructionScript)