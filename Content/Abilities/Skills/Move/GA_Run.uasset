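; GA_Run is a hold-to-run Gameplay Ability that raises the character's max walk speed while its input is held.
; On activation it commits, removes the State.RecoverStamina tag, boosts CharacterMovement speed and ends when WaitInputRelease fires.
; On end, a Sequence restores the lower speed immediately while a short Delay postpones re-adding the stamina recovery tag.
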(event Ability|EventActivateAbility
  (Ability|CommitAbility)
  (bind _asmy_character (Utilities|Casting|CastToMyCharacter (Ability|GetAvatarActorfromActorInfo)))
  (Class|MyCharacter|RemoveGameplayTags _asmy_character "(GameplayTags=((TagName=\"State.RecoverStamina\")))")
  (Variables|/Script/Engine.CharacterMovementComponent|SetMaxWalkSpeed (Variables|/Script/Engine.Character|GetCharacterMovement _asmy_character) 7e+02)
  (Ability|Tasks|WaitInputRelease false
    (:OnRelease
      (Ability|EndAbility))))

(event Ability|EventOnEndAbility
  (params (bWasCancelled :type Boolean))
  (Utilities|FlowControl|Sequence
    (:then_0
      (bind _asmy_character (Utilities|Casting|CastToMyCharacter (Ability|GetAvatarActorfromActorInfo)))
      (Utilities|FlowControl|Delay 0.6)
      (Class|MyCharacter|AddGameplayTags _asmy_character "(GameplayTags=((TagName=\"State.RecoverStamina\")))"))
    (:then_1
      (Variables|/Script/Engine.CharacterMovementComponent|SetMaxWalkSpeed (Variables|/Script/Engine.Character|GetCharacterMovement _asmy_character) 4.8e+02))))