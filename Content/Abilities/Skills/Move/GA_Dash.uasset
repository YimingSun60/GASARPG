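; GA_Dash is a Gameplay Ability that dashes the avatar along its forward vector.
; After a successful commit, it plays a sped-up montage and immediately applies a short constant root motion force, without waiting for the montage to finish.
; The force sets velocity on finish from the avatar's velocity, and its completion ends the ability.
; A failed commit cancels the ability.
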(event Ability|EventActivateAbility
  (bind _returnvalue (Ability|GetAvatarActorfromActorInfo))
  (bind _returnvalue_2 (Ability|CommitAbility))
  (if _returnvalue_2
    (Development|PrintString "Success")
    (|PlayMontageandWaitProxy "None" (Variables|Default|GetMontage%20to%20Play) 2.0 "None" true 1.0 0.0
      (:then
        (Ability|Tasks|ApplyRootMotionConstantForce "None" (Transformation|GetActorForwardVector _returnvalue) 3e+03 0.3 false 0 "SetVelocity" (Transformation|GetVelocity _returnvalue)
          (:OnFinish
            (Ability|EndAbility)))))
    (else
      (Ability|CancelAbility))))

(event Ability|EventOnEndAbility
  (params (bWasCancelled :type Boolean)))